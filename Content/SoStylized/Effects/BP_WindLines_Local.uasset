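; BP_WindLines_Local is an effect actor for stylized wind lines, driven by the NEWindLinesV2 effect component.
; Its construction script copies the actor's length and height ranges, spawn rate and opacity into the effect's user variables.
; It also converts the actor's yaw into a negated fraction of a full turn for Additional Rotation, so rotating the actor feeds into the effect's rotation.
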(fn `UserConstructionScript`
  (bind (_returnvalue_roll _returnvalue_pitch _returnvalue_yaw) (`KismetMathLibrary.BreakRotator` (`self.K2_GetActorRotation`)))
  (bind _ne_windlines_v2 (`self.NE_WindLines_v2`))
  (`NiagaraComponent.SetVariableFloat` _ne_windlines_v2 "Length Minimum" (`self.Wind Line Length Min`))
  (`NiagaraComponent.SetVariableFloat` _ne_windlines_v2 "Length Maximum" (`self.Wind Line Length Max`))
  (`NiagaraComponent.SetVariableFloat` _ne_windlines_v2 "Height Minimum" (`self.Wind Line Height Min`))
  (`NiagaraComponent.SetVariableFloat` _ne_windlines_v2 "Height Maximum" (`self.Wind Line Height Max`))
  (`NiagaraComponent.SetVariableFloat` _ne_windlines_v2 "Spawn Rate" (`self.Wind Spawn Rate`))
  (`NiagaraComponent.SetVariableFloat` _ne_windlines_v2 "Opacity" (`self.Wind Line Opacity`))
  (`NiagaraComponent.SetVariableFloat` _ne_windlines_v2 "Additional Rotation" (/ _returnvalue_yaw -360.0)))