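; BP_farmfence is a procedural farm fence actor that tiles a static mesh over an area sized by Roomvector.
; The construction script derives column and row counts from Roomvector's X and Y using fixed spacing per axis.
; Nested inclusive loops add an InstancedStaticMesh instance at each grid point, so even a zero size yields one piece.
; The event graph has no active logic.
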(fn `UserConstructionScript`
  (locals (`L width` :type Integer :default 0) (`L Depth` :type Integer :default 0) (`L width index` :type Integer) (`L depth index` :type Integer))
  (set `local.L width` (`KismetMathLibrary.FTrunc` (/ (.x (`self.roomvector`)) 216.0)))
  (set `local.L Depth` (`KismetMathLibrary.FTrunc` (/ (.y (`self.roomvector`)) 12.0)))
  (for _index (range (+ (`local.L width`) 1))
    (set `local.L width index` _index)
    (for _index_2 (range (+ (`local.L Depth`) 1))
      (set `local.L depth index` _index_2)
      (`InstancedStaticMeshComponent.AddInstance` (`self.InstancedStaticMesh`) (`KismetMathLibrary.MakeTransform` (`KismetMathLibrary.MakeVector` (`KismetMathLibrary.Conv_IntToDouble` (* (`local.L width index`) 216)) (`KismetMathLibrary.Conv_IntToDouble` (* (`local.L depth index`) 12)))) false))))